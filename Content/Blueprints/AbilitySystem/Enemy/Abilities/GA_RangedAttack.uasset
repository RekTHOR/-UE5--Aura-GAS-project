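; GA_RangedAttack is an enemy gameplay ability that fires a projectile at the avatar's combat target.
; On activation it turns the avatar toward the target and plays a random tagged attack montage from the avatar.
; A gameplay event matching that montage's tag triggers SpawnProjectile toward the target's location, syncing the shot to the animation.
; The ability ends when the montage completes, is interrupted or is cancelled.
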(event `self.K2_ActivateAbility`
  (bind _output_get (set `self.AvatarActor` (`self.GetAvatarActorFromActorInfo`)))
  (bind _returnvalue (message `EnemyInterface.GetCombatTarget` _output_get))
  (bind _returnvalue_2 (`Actor.K2_GetActorLocation` _returnvalue))
  (message `CombatInterface.SetFacingTarget` (`self.AvatarActor`) _returnvalue_2)
  (bind _returnvalue_3 (message `CombatInterface.GetAttackMontages` (`self.AvatarActor`)))
  (bind _output_get_2 (set `self.TaggedMontage` (`KismetArrayLibrary.Array_Random` _returnvalue_3)))
  (bind (_montage _montagetag) (break `TaggedMontage` _output_get_2))
  (`AbilityTask_PlayMontageAndWait.CreatePlayMontageAndWaitProxy` "None" _montage 1.0 "None" false
    (:`then`
      (`AbilityTask_WaitGameplayEvent.WaitGameplayEvent` _montagetag null
        (:`EventReceived`
          (message `CombatInterface.GetCombatSocketLocation` (`self.AvatarActor`) _montagetag)
          (`self.SpawnProjectile` _returnvalue_2))))
    (:`OnCompleted`
      (`self.K2_EndAbility` :!label _label))
    (:`OnInterrupted`
      (goto _label))
    (:`OnCancelled`
      (goto _label))))