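; Gameplay ability for enemy melee attacks, using the avatar's combat interface to face its combat target and play a random tagged attack montage.
; When the montage's tag event fires, it finds live players in a small sphere at the tagged socket and damages non-friends.
; A hit executes the MeleeImpact gameplay cue, passing the montage tag.
; The ability ends after that event or when the montage completes or is interrupted.
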(event `self.K2_ActivateAbility`
  (set `self.HasHitTarget` false)
  (set `self.AvatarActor` (`self.GetAvatarActorFromActorInfo`))
  (bind _returnvalue (message `EnemyInterface.GetCombatTarget` (`self.AvatarActor`)))
  (bind _ascombat_interface (cast `CombatInterface` (`self.AvatarActor`)))
  (`CombatInterface.SetFacingTarget` _ascombat_interface (`Actor.K2_GetActorLocation` _returnvalue))
  (bind _returnvalue_2 (message `CombatInterface.GetAttackMontages` (`self.AvatarActor`)))
  (bind _output_get (set `self.TaggedMontage` (`KismetArrayLibrary.Array_Random` _returnvalue_2)))
  (bind (_montage _montagetag _sockettag) (break `TaggedMontage` _output_get))
  (`AbilityTask_PlayMontageAndWait.CreatePlayMontageAndWaitProxy` "None" _montage
    (:`then`
      (`AbilityTask_WaitGameplayEvent.WaitGameplayEvent` _montagetag null
        (:`EventReceived`
          (bind _returnvalue_3 (message `CombatInterface.GetCombatSocketLocation` (`self.AvatarActor`) _sockettag))
          (bind _output_get_2 (set `self.CombatSocketLocation` _returnvalue_3))
          (bind _outoverlappingactors (`AuraAbilitySystemLibrary.GetLivePlayersWithinRadius` (`self.AvatarActor`) (`|MakeArray` (`self.AvatarActor`)) 45.0 _output_get_2))
          (for _array_element _outoverlappingactors
            (if (`AuraAbilitySystemLibrary.IsNotFriend` (`self.AvatarActor`) _array_element)
              (`self.CauseDamage` _array_element)
              (set `self.HasHitTarget` true)))
          (if (`self.HasHitTarget`)
            (bind _returnvalue_4 (message `EnemyInterface.GetCombatTarget` (`self.AvatarActor`)))
            (`self.K2_ExecuteGameplayCueWithParams` (struct :`TagName` "GameplayCue.MeleeImpact") (`AbilitySystemBlueprintLibrary.MakeGameplayCueParameters` 0.0 0.0 (struct) (struct) (struct) (`BlueprintGameplayTagLibrary.MakeGameplayTagContainerFromTag` (`.MontageTag` (break `TaggedMontage` (`self.TaggedMontage`)))) (struct) (`self.CombatSocketLocation`) (0.0 0.0 0.0) null (`self.AvatarActor`) _returnvalue_4)))
          (`self.K2_EndAbility`))))
    (:`OnCompleted`
      (`self.K2_EndAbility` :!label _label))
    (:`OnInterrupted`
      (goto _label))
    (:`OnCancelled`
      (goto _label))))