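; Melee attack gameplay ability that turns the avatar toward its combat target through the CombatInterface and plays a spear attack montage.
; While the montage plays, it waits for the spear attack gameplay event, then gets the combat socket location from the avatar.
; It draws a debug sphere at that location and ends, with no hit detection or damage applied yet.
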(event `self.K2_ActivateAbility`
  (bind _returnvalue (`self.GetAvatarActorFromActorInfo`))
  (bind _returnvalue_2 (message `EnemyInterface.GetCombatTarget` _returnvalue))
  (bind _ascombat_interface (cast `CombatInterface` _returnvalue))
  (`CombatInterface.SetFacingTarget` _ascombat_interface (`Actor.K2_GetActorLocation` _returnvalue_2))
  (`AbilityTask_PlayMontageAndWait.CreatePlayMontageAndWaitProxy` "None" "/Game/Assets/Enemies/Goblin/Animations/Spear/AM_SpearAttack.AM_SpearAttack"
    (:`then`
      (`AbilityTask_WaitGameplayEvent.WaitGameplayEvent` (struct :`TagName` "Event.Montage.SpearAttack") null
        (:`EventReceived`
          (bind _returnvalue_3 (message `CombatInterface.GetCombatSocketLocation` (`self.GetAvatarActorFromActorInfo`)))
          (`KismetSystemLibrary.DrawDebugSphere` _returnvalue_3 45.0 12 (struct :`R` 0.985917 :`G` 0.106283 :`B` 1.0 :`A` 1.0) 2.0)
          (`self.K2_EndAbility`))))))